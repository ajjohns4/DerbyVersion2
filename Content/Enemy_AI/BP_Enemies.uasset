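; Enemy character that fires a Wipeout blaster at the player's derby pawn and can be destroyed by damage.
; PawnSensing sightings of BP_Derby trigger a delayed projectile spawn from the Blaster component, marked as temporary.
; Damage updates a widget health bar that turns toward the camera each tick; at zero health the enemy calls EnemyEliminated, explodes and is destroyed.
; A kart-overlap sound is also wired, while older health bar and kill-count logic sits disconnected.
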(event `self.ReceiveTick`
  (params (DeltaSeconds :type "Float (single-precision)"))
  (`SceneComponent.K2_SetWorldRotation` (`self.health bar`) (`KismetMathLibrary.FindLookAtRotation` (`SceneComponent.K2_GetComponentLocation` (`self.health bar`)) (`SceneComponent.K2_GetComponentLocation` (`PlayerCameraManager.TransformComponent` (`GameplayStatics.GetPlayerCameraManager` 0)))) false false))

(event `self.Hit.OnComponentBeginOverlap`
  (params (OverlappedComponent :type "PrimitiveComponent Object Reference") (OtherActor :type "Actor Object Reference") (OtherComp :type "PrimitiveComponent Object Reference") (OtherBodyIndex :type Integer) (bFromSweep :type Boolean) (SweepResult :type "HitResult Structure (by ref)"))
  (castclass `/Game/BP/RevisedKartFunctions/Blueprints/New_BP_NewKart` (`GameplayStatics.GetObjectClass` OtherActor))
  (`GameplayStatics.PlaySound2D` "/Engine/EditorSounds/Notifications/CompileFailed.CompileFailed" 1.0 1.0 0.0 null null))

(event `self.PawnSensing.OnSeePawn`
  (params (Pawn :type "Pawn Object Reference"))
  ;[1 1 1] Wipeout Blaster(Temp)
  (cast `/Game/BP/RevisedKartFunctions/Blueprints/BP_Derby` Pawn)
  (`|ExecutionSequence`
    (:`then_1`
      (`KismetSystemLibrary.Delay` 1.5)
      (`GameplayStatics.PlaySoundAtLocation` "/Game/Assets/Sounds/BlasterCue.BlasterCue" (0.0 0.0 0.0) (struct) 0.5 1.0 0.0 null null null null)
      (`|SpawnActorFromClass` "/Game/BP/BP_Modified_WipeBlast.BP_Modified_WipeBlast_C" (`SceneComponent.K2_GetComponentToWorld` (`self.Blaster`)) "Undefined" "MultiplyWithRoot" null null))))

(event `self.ReceiveAnyDamage`
  (params (Damage :type "Float (single-precision)") (DamageType :type "DamageType Object Reference") (InstigatedBy :type "Controller Object Reference") (DamageCauser :type "Actor Object Reference"))
  ;[1 1 1] Enemy Health
  (set `self.enemy_Health` (- (`self.enemy_Health`) Damage))
  (bind _aswb_enemyhealth (cast `/Game/Enemy_AI/WB_enemyhealth` (`WidgetComponent.GetWidget` (`self.health bar`))))
  (`/Game/Enemy_AI/WB_enemyhealth.Updatehealthbar` _aswb_enemyhealth (`self.enemy_Health`))
  (if (<= (`self.enemy_Health`) 0.0)
    (`KismetSystemLibrary.PrintString` "dead")
    (`|ExecutionSequence`
      (:`then_0`
        (`self.EnemyEliminated`))
      (:`then_1`
        (`CharacterMovementComponent.DisableMovement` (`self.CharacterMovement`))
        (`GameplayStatics.PlaySound2D` "/Game/Assets/Sounds/Wipeout_Death.Wipeout_Death" 1.0 1.0 0.0 null null)
        (`KismetSystemLibrary.Delay` 0.1)
        (`NiagaraFunctionLibrary.SpawnSystemAtLocation` "/Game/Assets/VFX/WipeoutExplsoion.WipeoutExplsoion" (`self.K2_GetActorLocation`))
        (`self.K2_DestroyActor`)))
    (else
      (`KismetSystemLibrary.PrintString` (`KismetStringLibrary.Conv_DoubleToString` (`self.enemy_Health`))))))

(fn `UserConstructionScript`)