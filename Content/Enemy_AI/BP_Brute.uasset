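; BP_Brute is an enemy that fires on the player's BP_Derby and ends the encounter with a win screen when killed.
; Pawn sensing increments Derby's BruteCount and spawns BP_Modified_WipeBlast projectiles from two blasters after a delay, in logic marked temporary.
; Damage lowers EnemyHealth and updates a widget health bar that turns toward the camera every tick.
; At zero health it destroys itself and hands input to the win widget.
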(event `self.ReceiveTick`
  (params (DeltaSeconds :type "Float (single-precision)"))
  (`SceneComponent.K2_SetWorldRotation` (`self.health bar`) (`KismetMathLibrary.FindLookAtRotation` (`SceneComponent.K2_GetComponentLocation` (`self.health bar`)) (`SceneComponent.K2_GetComponentLocation` (`PlayerCameraManager.TransformComponent` (`GameplayStatics.GetPlayerCameraManager` 0)))) false false))

(event `self.Hit.OnComponentBeginOverlap`
  (params (OverlappedComponent :type "PrimitiveComponent Object Reference") (OtherActor :type "Actor Object Reference") (OtherComp :type "PrimitiveComponent Object Reference") (OtherBodyIndex :type Integer) (bFromSweep :type Boolean) (SweepResult :type "HitResult Structure (by ref)"))
  (castclass `/Game/BP/RevisedKartFunctions/Blueprints/BP_Derby` (`GameplayStatics.GetObjectClass` OtherActor))
  (`GameplayStatics.PlaySound2D` "/Engine/EditorSounds/Notifications/CompileFailed.CompileFailed" 1.0 1.0 0.0 null null))

(event `self.PawnSensing.OnSeePawn`
  (params (Pawn :type "Pawn Object Reference"))
  ;[1 1 1] Wipeout Blaster(Temp)
  (`self.Blaster2 Fire`)
  (cast `/Game/BP/RevisedKartFunctions/Blueprints/BP_Derby` Pawn)
  (`|ExecutionSequence`
    (:`then_0`
      (bind _asbp_derby (cast `/Game/BP/RevisedKartFunctions/Blueprints/BP_Derby` (`GameplayStatics.GetPlayerPawn` 0)))
      (`/Engine/EditorBlueprintResources/StandardMacros.IncrementInt` (`/Game/BP/RevisedKartFunctions/Blueprints/BP_Derby.bruteCount` _asbp_derby)))
    (:`then_1`
      (`KismetSystemLibrary.Delay` 2.0)
      (`GameplayStatics.PlaySoundAtLocation` "/Game/Assets/Sounds/BlasterCue.BlasterCue" (0.0 0.0 0.0) (struct) 1.0 1.0 0.0 null null null null)
      (`|SpawnActorFromClass` "/Game/BP/BP_Modified_WipeBlast.BP_Modified_WipeBlast_C" (`SceneComponent.K2_GetComponentToWorld` (`self.Blaster`)) "Undefined" "MultiplyWithRoot" null null))))

(event `Blaster2 Fire`
  ;[1 1 1] Wipeout Blaster(Temp)
  (cast `/Game/BP/RevisedKartFunctions/Blueprints/BP_Derby` (stale `self.PawnSensing.OnSeePawn` Pawn))
  (`KismetSystemLibrary.Delay` 2.0)
  (`GameplayStatics.PlaySoundAtLocation` "/Game/Assets/Sounds/BlasterCue.BlasterCue" (0.0 0.0 0.0) (struct) 1.0 1.0 0.0 null null null null)
  (`|SpawnActorFromClass` "/Game/BP/BP_Modified_WipeBlast.BP_Modified_WipeBlast_C" (`SceneComponent.K2_GetComponentToWorld` (`self.Blaster2`)) "Undefined" "MultiplyWithRoot" null null))

(event `self.ReceiveAnyDamage`
  (params (Damage :type "Float (single-precision)") (DamageType :type "DamageType Object Reference") (InstigatedBy :type "Controller Object Reference") (DamageCauser :type "Actor Object Reference"))
  ;[1 1 1] Enemy Health
  (set `self.enemy_Health` (- (`self.enemy_Health`) Damage))
  (bind _aswb_enemyhealth (cast `/Game/Enemy_AI/WB_enemyhealth` (`WidgetComponent.GetWidget` (`self.health bar`))))
  (`/Game/Enemy_AI/WB_enemyhealth.Updatehealthbar` _aswb_enemyhealth (`self.enemy_Health`))
  (if (<= (`self.enemy_Health`) 0.0)
    (`KismetSystemLibrary.PrintString` "dead")
    (`GameplayStatics.PlaySound2D` "/Game/Assets/Sounds/Wipeout_Death.Wipeout_Death" 1.0 1.0 0.0 null null)
    (`self.K2_DestroyActor`)
    (bind _returnvalue (`|CreateWidget` "/Game/UI/UI_Menus/WB_WinScreen.WB_WinScreen_C"))
    (`UserWidget.AddToViewport` _returnvalue 0)
    (`WidgetBlueprintLibrary.SetInputMode_UIOnlyEx` null _returnvalue)
    (`Widget.SetKeyboardFocus` (`/Game/UI/UI_Menus/WB_WinScreen.ReturnToHub_button` _returnvalue))
    (else
      (`KismetSystemLibrary.PrintString` (`KismetStringLibrary.Conv_DoubleToString` (`self.enemy_Health`))))))

(fn `UserConstructionScript`)