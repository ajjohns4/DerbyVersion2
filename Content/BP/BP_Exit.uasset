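; BP_Exit is an exit actor that shows an interaction widget while the player is near it.
; It creates a WB_A_Interact widget on BeginPlay, then adds it to the viewport when the player pawn enters its Box and removes it when the pawn leaves.
; The Blueprint only toggles the widget and holds no input handling or exit logic.
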(event `self.ReceiveBeginPlay`
  ;[1 1 1] Create widget
  (bind _returnvalue (`|CreateWidget` "/Game/DerbyAssets/Blueprints/MainMenu_UI/WB_A_Interact.WB_A_Interact_C"))
  (set `self.Interact_WIdget` _returnvalue))

(event `self.Box.OnComponentBeginOverlap`
  (params (OverlappedComponent :type "PrimitiveComponent Object Reference") (OtherActor :type "Actor Object Reference") (OtherComp :type "PrimitiveComponent Object Reference") (OtherBodyIndex :type Integer) (bFromSweep :type Boolean) (SweepResult :type "HitResult Structure (by ref)"))
  ;[1 1 1] Show Widget
  (if (== OtherActor (`GameplayStatics.GetPlayerPawn` 0))
    (`UserWidget.AddToViewport` (`self.Interact_WIdget`) 0)))

(event `self.Box.OnComponentEndOverlap`
  (params (OverlappedComponent :type "PrimitiveComponent Object Reference") (OtherActor :type "Actor Object Reference") (OtherComp :type "PrimitiveComponent Object Reference") (OtherBodyIndex :type Integer))
  ;[1 1 1] Show Widget
  (if (== (`GameplayStatics.GetPlayerPawn` 0) OtherActor)
    (`Widget.RemoveFromParent` (`self.Interact_WIdget`))))

(fn `UserConstructionScript`)