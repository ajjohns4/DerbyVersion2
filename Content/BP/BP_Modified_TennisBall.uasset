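; BP_Modified_TennisBall is a tennis ball actor that damages enemies on contact.
; Its Hitmarker overlap event casts the other actor to BP_Enemies, then BP_Brute, applying less damage to brutes, and ignores anything else.
; A hit prints a debug string, plays an impact sound at the world origin rather than the ball, and destroys the ball.
; A delayed self-destroy is present but unconnected, so it never runs.
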(event `self.Hitmarker.OnComponentBeginOverlap`
  (params (OverlappedComponent :type "PrimitiveComponent Object Reference") (OtherActor :type "Actor Object Reference") (OtherComp :type "PrimitiveComponent Object Reference") (OtherBodyIndex :type Integer) (bFromSweep :type Boolean) (SweepResult :type "HitResult Structure (by ref)"))
  ;[1 1 1] Tennis ball damage system
  (bind _asbp_enemies (cast `/Game/Enemy_AI/BP_Enemies` OtherActor)
    (:`then`
      (`KismetSystemLibrary.PrintString` "Damage")
      (`GameplayStatics.ApplyDamage` _asbp_enemies 0.5 null self)
      (`GameplayStatics.PlaySoundAtLocation` "/Game/Assets/Sounds/Wipeout_Impact.Wipeout_Impact" (0.0 0.0 0.0) (struct) 0.5 1.0 0.0 null null null null)
      (`self.K2_DestroyActor`))
    (:`CastFailed`
      (bind _asbp_brute (cast `/Game/Enemy_AI/BP_Brute` OtherActor))
      (`KismetSystemLibrary.PrintString` "Damage")
      (`GameplayStatics.ApplyDamage` _asbp_brute 0.1 null self)
      (`GameplayStatics.PlaySoundAtLocation` "/Game/Assets/Sounds/Wipeout_Impact.Wipeout_Impact" (0.0 0.0 0.0) (struct) 0.5 1.0 0.0 null null null null)
      (`self.K2_DestroyActor`))))

(fn `UserConstructionScript`)