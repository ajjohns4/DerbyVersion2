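; BP_Derby is the player's combat kart, with a tennis-ball launcher, damageable health, random barks, HUD and pause menu.
; Each tick, per-wheel line traces apply spring-like suspension and drive forces to KartCollider, scaled by eased input and SpeedModifier.
; Torque handles steering and drifting, with hold time choosing particle tiers and release boosts.
; Bound enemy, spawner and frisbee events update counters that trigger alert widgets and set SpawnBrute once both goals are met.
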(event `self.ReceiveActorBeginOverlap`
  (params (OtherActor :type "Actor Object Reference"))
  ;[1 1 1] BP_Derby
  (bind _asbp_enemies (cast `/Game/Enemy_AI/BP_Enemies` OtherActor))
  (`GameplayStatics.ApplyDamage` self 0.15 null _asbp_enemies)
  (`KismetSystemLibrary.Delay` 5.0))

(event `self.ReceiveBeginPlay`
  ;[1 1 1] BP_Derby
  ;;[1 1 1] Apply the input mapping context to the player controller, allowing specified inputs to correspond to actions. Then add the health bar widget, then the speedometer
  (`|ExecutionSequence`
    (:`then_0`
      (`EnhancedInputSubsystemInterface.AddMappingContext` (pcsubsystem `EnhancedInputLocalPlayerSubsystem` (`GameplayStatics.GetPlayerController` 0)) "/Game/BP/RevisedKartFunctions/Inputs/New_IMC_Vehicle.New_IMC_Vehicle" 0 (struct)))
    (:`then_1`
      (bind _returnvalue (`|CreateWidget` "/Game/DerbyAssets/Blueprints/MainMenu_UI/OptionsMenu_UI/WB_healthBar.WB_healthBar_C" (`GameplayStatics.GetPlayerController` 0)))
      (`UserWidget.AddToViewport` _returnvalue 0))
    (:`then_2`
      (bind _returnvalue_2 (`|CreateWidget` "/Game/UI/HUD/W_Speedometer.W_Speedometer_C" (`GameplayStatics.GetPlayerController` 0)))
      (`UserWidget.AddToViewport` _returnvalue_2 0))
    (:`then_3`
      (`self.Barking`))
    (:`then_4`
      ;;[1 1 1] Checks all enemies in the scene and fires off an event if they are eleminated
      (bind _outactors (`GameplayStatics.GetAllActorsOfClass` "/Game/Enemy_AI/BP_Enemies.BP_Enemies_C"))
      (for _array_element _outactors
        (add `/Game/Enemy_AI/BP_Enemies.EnemyEliminated` _array_element (delegate `OnEnemyKilled`))))
    (:`then_5`
      ;;[1 1 1] Enemy spawners need their own call since they are not initially spawning enemies into the scene
      (bind _outactors_2 (`GameplayStatics.GetAllActorsOfClass` "/Game/Enemy_AI/BP_WipeoutSpawner.BP_WipeoutSpawner_C"))
      (for _array_element_2 _outactors_2
        (add `/Game/Enemy_AI/BP_WipeoutSpawner.EnemySpawned` _array_element_2 (delegate `OnEnemySpawned`))))
    (:`then_6`
      ;;[1 1 1] Get for all items
      (bind _outactors_3 (`GameplayStatics.GetAllActorsOfClass` "/Game/BP/BP_frisbee.BP_frisbee_C"))
      (for _array_element_3 _outactors_3
        (add `/Game/BP/BP_frisbee.ItemCollected` _array_element_3 (delegate `OnItemCollected`))))))

(event `self.ReceiveAnyDamage`
  (params (Damage :type "Float (single-precision)") (DamageType :type "DamageType Object Reference") (InstigatedBy :type "Controller Object Reference") (DamageCauser :type "Actor Object Reference"))
  ;[1 1 1] BP_Derby
  ;;[1 1 1] Health
  (set `self.health` (- (`self.health`) Damage))
  (if (<= (`self.health`) 0.0)
    (`KismetSystemLibrary.PrintString` "dead")
    (`GameplayStatics.PlaySoundAtLocation` "/Game/Assets/Sounds/Gameover.Gameover" (0.0 0.0 0.0) (struct) 1.0 1.0 0.0 null null null null)
    (`KismetSystemLibrary.Delay` 5.0)
    (bind _returnvalue (`|CreateWidget` "/Game/UI/UI_Menus/WB_LoseScreen_V2.WB_LoseScreen_V2_C"))
    (`UserWidget.AddToViewport` _returnvalue 0)
    (else
      (`KismetSystemLibrary.PrintString` (`KismetStringLibrary.Conv_DoubleToString` (`self.health`))))))

(event `EnhancedInput|/Game/BP/RevisedKartFunctions/Inputs/New_IA_Accelerate`
  (params (ActionValue :type "Float (double-precision)") (ElapsedSeconds :type "Float (double-precision)") (TriggeredSeconds :type "Float (double-precision)") (InputAction :type "InputAction Object Reference" :default "/Game/BP/RevisedKartFunctions/Inputs/New_IA_Accelerate.New_IA_Accelerate"))
  ;[1 1 1] BP_Derby
  ;;[1 1 1] Upon using the inputs corresponding to acceleration(W,S, and the buttom face button of a controller), Change the value of the accerlation input to the corresponding value, using the Finterp node to ease in and out of motion
  (:`Triggered`
    (set `self.IsAccelerating?` true)
    (set `self.AccelerationInput` (`KismetMathLibrary.FInterpTo` (`self.AccelerationInput`) (`KismetMathLibrary.SelectFloat` ActionValue 0.0 (`self.IsOnGround`)) (`GameplayStatics.GetWorldDeltaSeconds`) 0.5)))
  (:`Canceled`
    (set `self.IsAccelerating?` false :!label _label))
  (:`Completed`
    (goto _label)))

(event `EnhancedInput|/Game/BP/RevisedKartFunctions/Inputs/IA_PauseMenu`
  (params (ActionValue :type Boolean) (ElapsedSeconds :type "Float (double-precision)") (TriggeredSeconds :type "Float (double-precision)") (InputAction :type "InputAction Object Reference" :default "/Game/BP/RevisedKartFunctions/Inputs/IA_PauseMenu.IA_PauseMenu"))
  ;[1 1 1] BP_Derby
  ;;[1 1 1] If Q is pushed and is pause menu open is false -> set is pause menu open to true, open the widget, set game mode to game and UI, and set game to pause. If true -> set is pause menu open to false, remove widget, unpause game, and change game mode to game only
  (:`Started`
    (if (not (`self.IsPauseMenuOpen`))
      (set `self.IsPauseMenuOpen` true)
      (bind _returnvalue (`|CreateWidget` "/Game/UI/UI_Menus/WB_PauseMenu.WB_PauseMenu_C"))
      (bind _output_get (set `self.PauseMenuWidget` _returnvalue))
      (`UserWidget.AddToViewport` _output_get 0)
      (`WidgetBlueprintLibrary.SetInputMode_GameAndUIEx` null (`self.PauseMenuWidget`))
      (`GameplayStatics.SetGamePaused` true)
      (else
        (set `self.IsPauseMenuOpen` false)
        (`Widget.RemoveFromParent` (`self.PauseMenuWidget`))
        (`GameplayStatics.SetGamePaused` false)
        (`WidgetBlueprintLibrary.SetInputMode_GameOnly` null)))))

(event `OnEnemyKilled`
  ;[1 1 1] BP_Derby
  ;;[1 1 1] Checks all enemies in the scene and fires off an event if they are eleminated
  (set `self.killCount` (+ (`self.killCount`) 1))
  (`self.CheckConditions`))

(event `EnhancedInput|/Game/BP/RevisedKartFunctions/Inputs/New_IA_Flip`
  (params (ActionValue :type "Float (double-precision)") (ElapsedSeconds :type "Float (double-precision)") (TriggeredSeconds :type "Float (double-precision)") (InputAction :type "InputAction Object Reference" :default "/Game/BP/RevisedKartFunctions/Inputs/New_IA_Flip.New_IA_Flip"))
  (bind (_returnvalue_roll _returnvalue_pitch _returnvalue_yaw) (`KismetMathLibrary.BreakRotator` (`self.K2_GetActorRotation`)))
  ;[1 1 1] BP_Derby
  ;;[1 1 1] If the kart happens to flip over, press the associate input to put it back on at its origin
  (:`Triggered`
    (`self.K2_SetActorRotation` (`KismetMathLibrary.MakeRotator` 0.0 0.0 _returnvalue_yaw) true)))

(event `Key|Gamepad_LeftShoulder`
  (params (Key :type "Key Structure"))
  ;[0.8198 1 0.2773] Drift
  ;;[1 1 1] On clicking a corresponding key the cart begins drifting
  (:`Pressed`
    (if (`self.IsAccelerating?`) :!label _label_2
      (set `self.IsDrifting?` true)))
  (:`Released`
    (set `self.IsDrifting?` false :!label _label_3)))

(event `Start Timer`
  ;[1 1 1] BP_Derby
  ;;[1 1 1] Timer
  (`KismetSystemLibrary.K2_SetTimerDelegate` (delegate `Start Timer`) 1.0)
  (if (== (`self.Seconds`) 0)
    (if (== (`self.Minutes`) 0)
      (`GameplayStatics.OpenLevel` "UI_MainMenu")
      (else
        (set `self.Seconds` 59)
        (set `self.Minutes` (- (`self.Minutes`) 1))))
    (else
      (set `self.Seconds` (- (`self.Seconds`) 1)))))

(event `OnEnemySpawned`
  (params (SpawnedEnemy :type "/Game/Enemy_AI/BP_Enemies Object Reference"))
  ;[1 1 1] BP_Derby
  ;;[1 1 1] Functions for enemies spawned from a spawner
  (add `/Game/Enemy_AI/BP_Enemies.EnemyEliminated` SpawnedEnemy (delegate `OnSpawnedEnemyKilled`)))

(event `EnhancedInput|/Game/BP/RevisedKartFunctions/Inputs/New_IA_Steer`
  (params (ActionValue :type "Float (double-precision)") (ElapsedSeconds :type "Float (double-precision)") (TriggeredSeconds :type "Float (double-precision)") (InputAction :type "InputAction Object Reference" :default "/Game/BP/RevisedKartFunctions/Inputs/New_IA_Steer.New_IA_Steer"))
  (bind _relativerotation_roll (`KismetMathLibrary.BreakRotator` (`SceneComponent.RelativeRotation` (`self.FL_Wheel`))))
  ;[1 1 1] BP_Derby
  ;;[1 1 1] Upon using the associated buttons for Steering(A,D, and the left thumbstick), apply a force in the direction of the input to the kart to make it turn
  (:`Triggered`
    (set `self.SteeringInput` ActionValue)
    (`PrimitiveComponent.AddTorqueInRadians` (`self.Kart_Collider`) (`KismetMathLibrary.MakeVector` 0.0 0.0 (* ActionValue 57000.0 (`self.AccelerationInput`))) "None" false)
    ;;[1 1 1] To rotate the front wheels to match the direction of the desired rotation, set the relative location in comparisons to the action value of the input
    (`SceneComponent.K2_SetRelativeRotation` (`self.FL_Wheel`) (`KismetMathLibrary.MakeRotator` 0.0 0.0 (`KismetMathLibrary.FInterpTo` _relativerotation_roll ActionValue (`GameplayStatics.GetWorldDeltaSeconds`) 3.0)) false false)
    (`SceneComponent.K2_SetRelativeRotation` (`self.FR_Wheel`) (`KismetMathLibrary.MakeRotator` 0.0 0.0 (`KismetMathLibrary.FInterpTo` _relativerotation_roll ActionValue (`GameplayStatics.GetWorldDeltaSeconds`) 3.0)) false false)))

(event `Key|SpaceBar`
  (params (Key :type "Key Structure"))
  ;[0.8198 1 0.2773] Drift
  ;;[1 1 1] On clicking a corresponding key the cart begins drifting
  (:`Pressed`
    (goto _label_2))
  (:`Released`
    (goto _label_3)))

(event `OnSpawnedEnemyKilled`
  ;[1 1 1] BP_Derby
  ;;[1 1 1] Functions for enemies spawned from a spawner
  (set `self.killCount` (+ (`self.killCount`) 1))
  (`self.CheckConditions`))

(event `OnItemCollected`
  ;[1 1 1] BP_Derby
  ;;[1 1 1] Get for all items
  (set `self.Amountofitems` (+ (`self.Amountofitems`) 1))
  (`self.CheckConditions`))

(event `Key|Gamepad_LeftShoulder`
  (params (Key :type "Key Structure"))
  ;[0.8198 1 0.2773] Drift
  ;;[1 1 1] Logic to Determine what direction the drift is applied. If you are steering left you will be drifting left, if you are steering right you will be drifitng right.
  (:`Pressed`
    (`KismetSystemLibrary.Delay` 0.25 :!label _label_4)
    (if (and (< (`self.SteeringInput`) 0.0) (`self.IsDrifting?`))
      (set `self.IsDriftingLeft?` true)
      (else
        (set `self.IsDriftingLeft?` false)
        (if (and (> (`self.SteeringInput`) 0.0) (`self.IsDrifting?`))
          (set `self.IsDriftingRight?` true)
          (else
            (set `self.IsDriftingRight?` false)))))))

(event `EnhancedInput|/Game/BP/RevisedKartFunctions/Inputs/IA_Drift`
  (params (ActionValue :type "Float (double-precision)") (ElapsedSeconds :type "Float (double-precision)") (TriggeredSeconds :type "Float (double-precision)") (InputAction :type "InputAction Object Reference" :default "/Game/BP/RevisedKartFunctions/Inputs/IA_Drift.IA_Drift"))
  (bind _kart_collider (`self.Kart_Collider`))
  (bind _kart_collider_2 (`self.Kart_Collider`))
  ;[0.8198 1 0.2773] Drift
  (:`Triggered`
    ;;[1 1 1] If the vechicle is drifitng left, do a continous check to determine whether the player is holding the buttons associated to steering left and right. Depending on this factor increase the "tightness" of the turning angle to compensate for players direction
    (if (`self.IsDriftingLeft?`) :!label _label_5
      (if (< (`self.SteeringInput`) 0.0)
        (`PrimitiveComponent.AddTorqueInRadians` (`self.Kart_Collider`) (0.0 0.0 -250000.0) "None" false)
        (elif (> (`self.SteeringInput`) 0.0)
          (`PrimitiveComponent.AddTorqueInRadians` (`self.Kart_Collider`) (0.0 0.0 -100000.0) "None" false)
          (else
            (`PrimitiveComponent.AddTorqueInRadians` (`self.Kart_Collider`) (0.0 0.0 -12500.0) "None" false))))
      ;;[1 1 1] All "Torque in Radians nodes" feeding into a branch checking if the drift has been cancelled. If the druft has been cancelled, break the loop of adding force at the new angle of the turn
      (if (`self.DriftCancel`) :!label _label_6
        (goto _label_7 :!via `Break`)
        (else
          ;;[1 1 1] All "Torque in Radians nodes" feeding into a branch checking if the drift has not been cancelled. If the druft has been cancelled, break the loop of adding force at the new angle of the turn for if the kart is driftng right
          (if (not (not (`self.DriftCancel`)))
            (goto _label_8 :!via `Break`))))
      (else
        ;;[1 1 1] If the vechicle is drifitng right, do a continous check to determine whether the player is holding the buttons associated to steering left and right. Depending on this factor increase the "tightness" of the turning angle to compensate for players direction
        (if (`self.IsDriftingRight?`)
          (if (> (`self.SteeringInput`) 0.0)
            (`PrimitiveComponent.AddTorqueInRadians` (`self.Kart_Collider`) (0.0 0.0 250000.0) "None" false)
            (goto _label_6)
            (elif (< (`self.SteeringInput`) 0.0)
              (`PrimitiveComponent.AddTorqueInRadians` (`self.Kart_Collider`) (0.0 0.0 100000.0) "None" false)
              (goto _label_6)
              (else
                (`PrimitiveComponent.AddTorqueInRadians` (`self.Kart_Collider`) (0.0 0.0 12500.0) "None" false)
                (goto _label_6))))))))
  (:`Started`
    ;;[1 1 1] On the start of the input being pressed ensure the druft is cancelled. If the input is released earlier than intended the drift will become cancelled and no logic will be applied
    (set `self.DriftCancel` false)
    (if (`self.IsDriftingLeft?`)
      (for _ (range 1) :!label _label_7
        ;;[1 1 1] As long as the kart is drifting, apply a force to rotate the kart in the new angle of the forward vector calculated in the previous step(where torque was applied to the kart.)
        (`PrimitiveComponent.AddForceAtLocation` _kart_collider (`KismetMathLibrary.GetForwardVector` (`SceneComponent.GetSocketRotation` _kart_collider "None")) (`SceneComponent.K2_GetComponentLocation` _kart_collider) "None"))
      (elif (`self.IsDriftingRight?`)
        (for _ (range 1) :!label _label_8
          ;;[1 1 1] As long as the kart is drifting, apply a force to rotate the kart in the new angle of the forward vector calculated in the previous step(where torque was applied to the kart.) The negative one ensures the force is applied in the opposite direction sinc the player is drifting to the right
          (`PrimitiveComponent.AddForceAtLocation` _kart_collider_2 (`KismetMathLibrary.GetForwardVector` (* (`SceneComponent.GetSocketRotation` _kart_collider_2 "None") -1.0)) (`SceneComponent.K2_GetComponentLocation` _kart_collider_2) "None")))))
  (:`Ongoing`
    (goto _label_5))
  (:`Canceled`
    (set `self.DriftCancel` true))
  (:`Completed`
    (set `self.IsDriftingLeft?` false)
    (set `self.IsDriftingRight?` false)
    (set `self.IsDrifting?` false)))

(event `Barking`
  ;[1 1 1] BP_Derby
  ;;[1 1 1] Derby Bark
  (`KismetSystemLibrary.Delay` (`KismetMathLibrary.RandomFloatInRange` 1.0 20.0))
  (`GameplayStatics.PlaySound2D` "/Game/Assets/Sounds/DerbyBarkCue.DerbyBarkCue" 1.0 1.0 0.0 null null)
  (`self.Barking`))

(event `Key|SpaceBar`
  (params (Key :type "Key Structure"))
  ;[0.8198 1 0.2773] Drift
  ;;[1 1 1] Logic to Determine what direction the drift is applied. If you are steering left you will be drifting left, if you are steering right you will be drifitng right.
  (:`Pressed`
    (goto _label_4)))

(event `CheckConditions`
  ;[1 1 1] BP_Derby
  (if (and (>= (`self.killCount`) 10) (>= (`self.Amountofitems`) 3) (== (`self.Collected_all_check?`) 0))
    (set `self.Collected_all_check?` 1)
    (bind _returnvalue (`|CreateWidget` "/Game/Assets/Widgets/Stage1/WB_CollectedAll.WB_CollectedAll_C"))
    (`UserWidget.AddToViewport` _returnvalue 0)
    (`KismetSystemLibrary.Delay` 2.3)
    (`Widget.RemoveFromParent` _returnvalue)
    (bind _returnvalue_2 (`|CreateWidget` "/Game/Assets/Widgets/Hub/WB_BruteAlert.WB_BruteAlert_C"))
    (`UserWidget.AddToViewport` _returnvalue_2 0)
    (`KismetSystemLibrary.Delay` 3.5)
    (`Widget.RemoveFromParent` _returnvalue_2)
    (set `self.SpawnBrute?` true)))

(event `StartShooting`
  (bind (_returnvalue_location _returnvalue_rotation) (`KismetMathLibrary.BreakTransform` (`SceneComponent.K2_GetComponentToWorld` (`self.TennisBallSpawn`))))
  (bind (_returnvalue_location_2 _returnvalue_rotation_2) (`KismetMathLibrary.BreakTransform` (`SceneComponent.K2_GetComponentToWorld` (`self.TennisBallSpawn`))))
  ;[1 1 1] BP_Derby
  ;;[1 1 1] Temp code for Derby's Launcher
  (set `self.isFiring` true)
  (`KismetSystemLibrary.Delay` (`self.fireRate`))
  (set `self.isFiring` false)
  (`GameplayStatics.PlaySoundAtLocation` "/Game/Assets/Sounds/Launcher_2.Launcher_2" (0.0 0.0 0.0) (struct) 1.0 1.0 0.0 null null null null)
  (bind _returnvalue (`NiagaraFunctionLibrary.SpawnSystemAtLocation` "/Game/Assets/VFX/BallSmoke.BallSmoke" _returnvalue_location _returnvalue_rotation (0.5 0.5 0.5)))
  (`KismetSystemLibrary.Delay` 0.5)
  (`ActorComponent.K2_DestroyComponent` _returnvalue)
  (`|SpawnActorFromClass` "/Game/BP/BP_Modified_TennisBall.BP_Modified_TennisBall_C" (`KismetMathLibrary.MakeTransform` _returnvalue_location_2 _returnvalue_rotation_2 (0.5 0.5 0.5)) "AlwaysSpawn" "MultiplyWithRoot" null 10000.0 0.0 null))

(event `self.ReceiveTick`
  (params (DeltaSeconds :type "Float (single-precision)"))
  ;[1 1 1] BP_Derby
  ;;[1 1 1] Every Frame create the suspension effect at each of the wheels using the created Suspension Cast Function
  (`self.SuspensionCast` (`self.FL_Wheel`))
  (`self.SuspensionCast` (`self.FR_Wheel`))
  (`self.SuspensionCast` (`self.BL_Wheel`))
  (`self.SuspensionCast` (`self.BR_Wheel`))
  ;;[1 1 1] Caculate the Accerleration which needs to be applied using the Caculate Acceleration Function
  (`self.CaculateAcceleration`)
  (bind _outhit (`KismetSystemLibrary.LineTraceSingle` (`SceneComponent.K2_GetComponentLocation` (`self.Camera`)) (`SceneComponent.K2_GetComponentLocation` (`self.Kart_Collider`)) "TraceTypeQuery2"))
  ;;[1 1 1] Updates Speedometer if player bounces off an obstacle preventing weird visuals
  (if (`self.HasBounced`)
    (if (<= (`self.CoolDownTimer`) 0.0)
      (set `self.HasBounced` false)
      (else
        (set `self.CoolDownTimer` (- (`self.CoolDownTimer`) 0.1))))
    (else
      (bind _output_get (set `self.CurrentVelocity` (`self.GetVelocity`)))
      (set `self.SmoothedVelocity` (`KismetMathLibrary.VLerp` _output_get (`self.PreviousframeSpeed`) 0.1))
      (set `self.PreviousframeSpeed` (`self.CurrentVelocity`)))))

(event `Key|LeftMouseButton`
  (params (Key :type "Key Structure"))
  ;[1 1 1] BP_Derby
  ;;[1 1 1] Temp code for Derby's Launcher
  (:`Pressed`
    (if (not (`self.isFiring`)) :!label _label_9
      (bind _returnvalue (`KismetSystemLibrary.K2_SetTimerDelegate` (delegate `StartShooting`) (`self.fireRate`) true))
      (`self.StartShooting`)))
  (:`Released`
    (`KismetSystemLibrary.K2_ClearAndInvalidateTimerHandle` _returnvalue :!label _label_10)))

(event `Key|Gamepad_FaceButton_Left`
  (params (Key :type "Key Structure"))
  ;[1 1 1] BP_Derby
  ;;[1 1 1] Temp code for Derby's Launcher
  (:`Pressed`
    (goto _label_9))
  (:`Released`
    (goto _label_10)))

(event `EnhancedInput|/Game/ThirdPerson/Input/Actions/IA_Reset_cam`
  (params (ActionValue :type Boolean) (ElapsedSeconds :type "Float (double-precision)") (TriggeredSeconds :type "Float (double-precision)") (InputAction :type "InputAction Object Reference" :default "/Game/ThirdPerson/Input/Actions/IA_Reset_cam.IA_Reset_cam"))
  (bind _returnvalue (`GameplayStatics.GetPlayerController` 0))
  ;[1 1 1] BP_Derby
  ;;[1 1 1] Camera
  (:`Started`
    (bind (_direction _resettrack) (`Timeline|reset cam` :!via `PlayFromStart`)
      (:`Update`
        (`Controller.SetControlRotation` _returnvalue (`KismetMathLibrary.RLerp` (`Controller.GetControlRotation` _returnvalue) (`SceneComponent.K2_GetComponentRotation` (`self.camera positon reference`)) _resettrack true))))))

(event `EnhancedInput|/Game/BP/RevisedKartFunctions/Inputs/IA_Drift`
  (params (ActionValue :type "Float (double-precision)") (ElapsedSeconds :type "Float (double-precision)") (TriggeredSeconds :type "Float (double-precision)") (InputAction :type "InputAction Object Reference" :default "/Game/BP/RevisedKartFunctions/Inputs/IA_Drift.IA_Drift"))
  ;[0.8198 1 0.2773] Drift
  ;;[1 1 1] Create different colored drifting particles depending on how long the drift input is held down
  (:`Triggered`
    (if (or (`self.IsDriftingRight?`) (`self.IsDriftingLeft?`)) :!label _label_11
      (if (<= ElapsedSeconds 2.0)
        (`|ExecutionSequence`
          (:`then_0`
            (`|SpawnActorFromClass` "/Game/DerbyAssets/Niagra/BP_Low_Drift_Particles.BP_Low_Drift_Particles_C" (`KismetMathLibrary.Conv_VectorToTransform` (`SceneComponent.K2_GetComponentLocation` (`self.BR_Wheel`))) "AlwaysSpawn" "MultiplyWithRoot" null null))
          (:`then_1`
            (`|SpawnActorFromClass` "/Game/DerbyAssets/Niagra/BP_Low_Drift_Particles.BP_Low_Drift_Particles_C" (`KismetMathLibrary.Conv_VectorToTransform` (`SceneComponent.K2_GetComponentLocation` (`self.BL_Wheel`))) "AlwaysSpawn" "MultiplyWithRoot" null null)))
        (elif (<= ElapsedSeconds 4.0)
          (`|ExecutionSequence`
            (:`then_0`
              (`|SpawnActorFromClass` "/Game/DerbyAssets/Niagra/BP_Medium_Drift_Particles.BP_Medium_Drift_Particles_C" (`KismetMathLibrary.Conv_VectorToTransform` (`SceneComponent.K2_GetComponentLocation` (`self.BR_Wheel`))) "AlwaysSpawn" "MultiplyWithRoot" null null))
            (:`then_1`
              (`|SpawnActorFromClass` "/Game/DerbyAssets/Niagra/BP_Medium_Drift_Particles.BP_Medium_Drift_Particles_C" (`KismetMathLibrary.Conv_VectorToTransform` (`SceneComponent.K2_GetComponentLocation` (`self.BL_Wheel`))) "AlwaysSpawn" "MultiplyWithRoot" null null)))
          (else
            (`|ExecutionSequence`
              (:`then_0`
                (`|SpawnActorFromClass` "/Game/DerbyAssets/Niagra/BP_High_Drift_Particles.BP_High_Drift_Particles_C" (`KismetMathLibrary.Conv_VectorToTransform` (`SceneComponent.K2_GetComponentLocation` (`self.BR_Wheel`))) "AlwaysSpawn" "MultiplyWithRoot" null null))
              (:`then_1`
                (`|SpawnActorFromClass` "/Game/DerbyAssets/Niagra/BP_High_Drift_Particles.BP_High_Drift_Particles_C" (`KismetMathLibrary.Conv_VectorToTransform` (`SceneComponent.K2_GetComponentLocation` (`self.BL_Wheel`))) "AlwaysSpawn" "MultiplyWithRoot" null null))))))))
  (:`Ongoing`
    (goto _label_11))
  (:`Completed`
    ;;[1 1 1] When the input is released. ensuring the kart is no longer in the drift state.
    (set `self.IsDriftingRight?` false)
    (set `self.IsDriftingLeft?` false)
    ;;[1 1 1] If the inout associated with the drifitng is held for a desired amount of time, on release of the input apply the boost kart function to give the player a speed boost
    (if (>= ElapsedSeconds 4.0)
      (`self.BoostKart` 1.7 0.75)
      (elif (and (>= ElapsedSeconds 2.0) (< ElapsedSeconds 4.0))
        (`self.BoostKart` 1.4 0.75)))))

(event `EnhancedInput|/Game/ThirdPerson/Input/Actions/IA_FreeLook`
  (params (ActionValue :type "Vector2D Structure") (ElapsedSeconds :type "Float (double-precision)") (TriggeredSeconds :type "Float (double-precision)") (InputAction :type "InputAction Object Reference" :default "/Game/ThirdPerson/Input/Actions/IA_FreeLook.IA_FreeLook"))
  ;[1 1 1] BP_Derby
  ;;[1 1 1] Camera
  (:`Triggered`
    (`self.AddControllerYawInput` ActionValue_X)
    (`self.AddControllerPitchInput` ActionValue_Y)))

(event `self.Kart_Collider.OnComponentHit`
  (params (HitComponent :type "PrimitiveComponent Object Reference") (OtherActor :type "Actor Object Reference") (OtherComp :type "PrimitiveComponent Object Reference") (NormalImpulse :type "Vector Structure") (Hit :type "HitResult Structure (by ref)"))
  (bind (_bblockinghit _binitialoverlap _time _distance _location _impactpoint _normal _impactnormal _physmat _hitactor _hitcomponent) (`GameplayStatics.BreakHitResult` Hit))
  ;[0.8198 1 0.2773] Drift
  ;;[1 1 1] If the player collides with an object with the tag "Prop" apply a force to the player to act as if they are bouncing off the object
  (if (`ActorComponent.ComponentHasTag` _hitcomponent "Prop")
    (`PrimitiveComponent.AddImpulse` (`self.Kart_Collider`) (* (`KismetMathLibrary.MakeVector` (.x _impactnormal) (.y _impactnormal) (`KismetMathLibrary.FClamp` (.z _impactnormal) 0.0 0.0)) (30000.0 0.0 0.0)) "None" false)
    (set `self.HasBounced` true)
    (set `self.CoolDownTimer` 0.75)))

(fn `AccelerateKart`
  (params (WheelComp :type "SceneComponent Object Reference"))
  (bind _kart_collider (`self.Kart_Collider`))
  ;[1 1 1] Add an accerlation force in the direction of the forward vector(the front) of the object, allowing the kart to move forward. Select Vector changes the falling rate(i.e.) the gravity
  (`PrimitiveComponent.AddForceAtLocation` _kart_collider (+ (* (`SceneComponent.GetForwardVector` _kart_collider) 2500.0 (`self.AccelerationInput`) (`PrimitiveComponent.GetMass` _kart_collider) (`self.SpeedModifier`)) (`KismetMathLibrary.SelectVector` (0.0 0.0 0.0) (0.0 0.0 -5000.0) (`self.IsOnGround`))) (`SceneComponent.K2_GetComponentLocation` WheelComp) "None"))

(fn `BoostKart`
  (params (SpeedModifier :type "Float (single-precision)") (Time :type "Float (single-precision)"))
  ;[1 1 1] Change the speed modifer of the player, increasing their speed by a multiplier. This speed boost expires after a defined amount of time(which is defined in the kart's blueprint)
  (set `self.SpeedModifier` SpeedModifier)
  (`KismetSystemLibrary.K2_SetTimer` null "ResetSpeed" Time))

(fn `CaculateAcceleration`
  (bind _accelerationinput (`self.AccelerationInput`))
  ;[1 1 1] To preventprovide and cap speed ramping, the acceleration value is placed against the vaule given to the input, with is either postive or negative according to the direction held(The value of Acceleration will continously go up and down). This also allows for the object to ease out of its speed once the input is released
  (bind _output_get (set `self.Acceleration` (* (`KismetMathLibrary.Lerp` 0.0 15000.0 _accelerationinput) _accelerationinput)))
  (set `self.AccelerationInput` (`KismetMathLibrary.FInterpTo` (`self.AccelerationInput`) 0.0 (`GameplayStatics.GetWorldDeltaSeconds`) 0.4))
  ;[1 1 1] Add rotation to the wheels
  (`SceneComponent.K2_AddLocalRotation` (`self.Wheel_BR`) (`KismetMathLibrary.MakeRotator` (/ _output_get -1000.0)) false false)
  (`SceneComponent.K2_AddLocalRotation` (`self.Wheel_BL`) (`KismetMathLibrary.MakeRotator` (/ _output_get -1000.0)) false false)
  (`SceneComponent.K2_AddLocalRotation` (`self.Wheel_FR`) (`KismetMathLibrary.MakeRotator` (/ _output_get -1000.0)) false false)
  (`SceneComponent.K2_AddLocalRotation` (`self.Wheel_FL`) (`KismetMathLibrary.MakeRotator` (/ _output_get -1000.0)) false false))

(fn `IsOnGround`
  (returns (ReturnValue :type Boolean))
  (bind _returnvalue (`self.K2_GetActorLocation`))
  ;[1 1 1] Creates a line trace from the center of the wheel to determine if the kart is touching the ground
  (bind (_outhit _returnvalue_2) (`KismetSystemLibrary.LineTraceSingle` _returnvalue (- _returnvalue (0.0 0.0 60.0)) "TraceTypeQuery1"))
  (return _returnvalue_2))

(fn `randomBark`)

(fn `ResetSpeed`
  ;[1 1 1] Resets the speed modifier after interacting with a boostpad
  (set `self.SpeedModifier` 1.0))

(fn `SlipReduction`
  ;[1 1 1] By Applying A counter force to the kart when its turning, we can lower the kart natural ability to drift. Making turns more wide and less reponsive, put in place the potiential for an actual Drift mechanic
  (`PrimitiveComponent.AddForce` (`self.Kart_Collider`) (* (`SceneComponent.GetRightVector` (`self.Kart_Collider`)) (* (`KismetMathLibrary.Dot_VectorVector` (`SceneComponent.GetRightVector` (`self.Kart_Collider`)) (`SceneComponent.GetComponentVelocity` (`self.Kart_Collider`))) -100.0)) "None" false))

(fn `SuspensionCast`
  (params (WheelComp :type "SceneComponent Object Reference"))
  (bind _returnvalue (`SceneComponent.K2_GetComponentLocation` WheelComp))
  (bind _returnvalue_2 (`SceneComponent.GetChildComponent` (`local.WheelComp`) 0))
  (bind (_relativelocation_x _relativelocation_y _relativelocation_z) (`KismetMathLibrary.BreakVector` (`SceneComponent.RelativeLocation` _returnvalue_2)))
  ;[1 1 1] Create a line cast spanning from the center of an object(in this case the wheels) to a desired amount below(-60 in this case)
  (bind _outhit (`KismetSystemLibrary.LineTraceSingle` _returnvalue (+ _returnvalue (* (`SceneComponent.GetUpVector` WheelComp) -20.0)) "TraceTypeQuery1"))
  (bind (_bblockinghit _binitialoverlap _time _distance _location _impactpoint _normal _impactnormal _physmat _hitactor _hitcomponent _hitbonename _bonename _hititem _elementindex _faceindex _tracestart _traceend) (`GameplayStatics.BreakHitResult` _outhit))
  ;[1 1 1] If the line trace comes into contact with an object, apply upward propulsion(to create a suspension effect) to the collider at the location of the wheels
  (if _bblockinghit
    (`PrimitiveComponent.AddForceAtLocation` (`self.Kart_Collider`) (* (- 1.0 (`KismetMathLibrary.NormalizeToRange` _distance 0.0 20.0)) (`KismetMathLibrary.GetDirectionUnitVector` _traceend _tracestart) 22000.0) (`SceneComponent.K2_GetComponentLocation` (`local.WheelComp`)) "None")
    ;[1 1 1] Apply accerlation to the wheels using the Accerlerate Kart Function
    (`self.AccelerateKart` (`local.WheelComp`))
    ;[1 1 1] Specifically alter the wheels transformation to conform to the suspension values
    (`SceneComponent.K2_SetRelativeLocation` _returnvalue_2 (`KismetMathLibrary.MakeVector` 0.0 0.0 (`KismetMathLibrary.FInterpTo` _relativelocation_z (+ (* _distance -1.0) 11.5) (`GameplayStatics.GetWorldDeltaSeconds`) 3.0)) false false)
    (else
      (`self.AccelerateKart` (`local.WheelComp`)))))

(fn `UserConstructionScript`)