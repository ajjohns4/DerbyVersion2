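; GM_Derby is the game mode for a kart derby, seeding the level with frisbee pickups when play begins.
; SpawnItem picks three random BP_ItemSpawnPoint actors, spawns a BP_frisbee at each location, then removes and destroys that point so it is not reused.
; An uncalled Counter function reads the player's BP_Derby item and kill counts to set a timer's looping flag, but binds no event.
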(event `self.ReceiveBeginPlay`
  ;[1 1 1] Win Condition
  (`self.SpawnItem`))

(fn `Counter`
  (bind _asbp_derby (cast `/Game/BP/RevisedKartFunctions/Blueprints/BP_Derby` (`GameplayStatics.GetPlayerPawn` 0)))
  (`KismetSystemLibrary.K2_SetTimerDelegate` :`Time` 3.0 :`bLooping` (and (== (`/Game/BP/RevisedKartFunctions/Blueprints/BP_Derby.Amountofitems` _asbp_derby) 1) (== (`/Game/BP/RevisedKartFunctions/Blueprints/BP_Derby.killCount` _asbp_derby) 1))))

(fn `SpawnItem`
  (locals (localSpawnPoints :type "Array of /Game/BP/BP_ItemSpawnPoint Object Reference") (localItem :type "/Game/BP/BP_ItemSpawnPoint Object Reference"))
  ;[1 1 1] SpawnerSystem
  (bind _outactors (`GameplayStatics.GetAllActorsOfClass` "/Game/BP/BP_ItemSpawnPoint.BP_ItemSpawnPoint_C"))
  (set `local.localSpawnPoints` _outactors)
  (for _ (range 3)
    (set `local.localItem` (`KismetArrayLibrary.Array_Random` (`local.localSpawnPoints`)))
    (`|SpawnActorFromClass` "/Game/BP/BP_frisbee.BP_frisbee_C" (`KismetMathLibrary.MakeTransform` (`self.K2_GetActorLocation` (`local.localItem`))) "AdjustIfPossibleButAlwaysSpawn" "MultiplyWithRoot" null null)
    (`KismetArrayLibrary.Array_RemoveItem` (`local.localSpawnPoints`) (`local.localItem`))
    (`self.K2_DestroyActor` (`local.localItem`))))

(fn `UserConstructionScript`)